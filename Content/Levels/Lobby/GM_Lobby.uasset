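; Lobby game mode that manages joining players and gives each a pawn of their selected character.
; PostLogin tracks controllers and, after a retriggerable delay, kicks those beyond session capacity, updates the session, then spawns and possesses pawns for PC_Lobby controllers not yet set up.
; CreatActor maps the selection to the Ninja or ThirdPerson character at a player start.
; DebugMode skips session handling and spawns once two players are present; logout removes controllers.
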(event EventPostLogin
  (params (NewPlayer :type Player%20Controller%20Object%20Reference))
  (if (not (Variables|Default|GetDebugMode))
    ;[1 1 1] OnLogin (serveur)
    (Utilities|Array|AddUnique (Variables|Default|GetplayerControllers) NewPlayer)
    (Utilities|FlowControl|RetriggerableDelay 2.0)
    (bind (_numconnections _numprivateconnections _bislan _bisdedicated _ballowinvites _ballowjoininprogress _bisanticheatenabled _builduniqueid _extrasettings) (Class|AdvancedSessionsLibrary|GetSessionSettings)
      (:OnSuccess
        (if (> (Utilities|Array|Length (Variables|/Script/Engine.GameStateBase|GetPlayerArray (Game|GetGameState))) _numconnections)
          (bind (_arrayindex _arrayelement) (Utilities|Array|ReverseforEachLoop (Variables|Default|GetplayerControllers))
            (:LoopBody
              (if (>= _arrayindex _numconnections)
                (Class|AdvancedSessionsLibrary|KickPlayer _arrayelement "Server Full")))
            (:Completed
              (|UpdateSession _extrasettings _numconnections _numprivateconnections _bislan _ballowinvites _ballowjoininprogress true _bisdedicated :!label _label
                (:OnSuccess
                  (for _array_element (Variables|Default|GetplayerControllers)
                    (bind _aspc_lobby (Utilities|Casting|CastToPC_Lobby _array_element))
                    (if (not (Variables|/Game/Levels/Lobby/PC_Lobby.PC_Lobby_C|GetIsControllerSetUP _aspc_lobby))
                      (bind _bp_tpc (CallFunction|CreatActor (Variables|/Game/Levels/Lobby/PC_Lobby.PC_Lobby_C|GetCharacterSelection _aspc_lobby) (Transformation|GetActorTransform (Class|GameModeBase|FindPlayerStart _array_element "0"))))
                      (Pawn|Possess _aspc_lobby _bp_tpc)
                      (Variables|/Game/Levels/Lobby/PC_Lobby.PC_Lobby_C|SetIsControllerSetUP _aspc_lobby true)))))))
          (else
            (goto _label)))))
    (else
      (Utilities|Array|AddUnique (Variables|Default|GetplayerControllers) NewPlayer)
      (if (== (Utilities|Array|Length (Variables|/Script/Engine.GameStateBase|GetPlayerArray (Game|GetGameState))) 2)
        (for _array_element_2 (Variables|Default|GetplayerControllers)
          (bind _aspc_lobby_2 (Utilities|Casting|CastToPC_Lobby _array_element_2))
          (if (not (Variables|/Game/Levels/Lobby/PC_Lobby.PC_Lobby_C|GetIsControllerSetUP _aspc_lobby_2))
            (bind _bp_tpc_2 (CallFunction|CreatActor (Variables|/Game/Levels/Lobby/PC_Lobby.PC_Lobby_C|GetCharacterSelection _aspc_lobby_2) (Transformation|GetActorTransform (Class|GameModeBase|FindPlayerStart _array_element_2 "0"))))
            (Pawn|Possess _aspc_lobby_2 _bp_tpc_2)
            (Variables|/Game/Levels/Lobby/PC_Lobby.PC_Lobby_C|SetIsControllerSetUP _aspc_lobby_2 true)))))))

(event EventOnLogout
  (params (ExitingController :type Controller%20Object%20Reference))
  ;[1 1 1] OnLogout or OnKick
  (bind _asplayer_controller (Utilities|Casting|CastToPlayerController ExitingController))
  (Utilities|Array|RemoveItem (Variables|Default|GetplayerControllers) _asplayer_controller))

(fn ConstructionScript)

(fn CreatActor
  (params (Enum :type ENUM_Player_character_selection%20Enum :default "NewEnumerator0") (Transform :type Transform))
  (Utilities|FlowControl|Sequence
    (:then_0
      (if (Utilities|Enum|Equal(Enum) Enum "NewEnumerator0")
        (bind _returnvalue (Game|SpawnActorfromClass "/Game/ThirdPersonBP/BP_TPC_Ninja.BP_TPC_Ninja_C" Transform "Undefined" 0 0))
        (return _returnvalue)))
    (:then_1
      (if (Utilities|Enum|Equal(Enum) Enum "NewEnumerator1")
        (bind _returnvalue_2 (Game|SpawnActorfromClass "/Game/ThirdPersonBP/ThirdPersonCharacter.ThirdPersonCharacter_C" Transform "Undefined" 0 0))
        (return _returnvalue_2)))))