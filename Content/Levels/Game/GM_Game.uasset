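; Game mode for the game level that tracks joining and leaving players and spawns their selected characters.
; On player start, a retriggerable delay precedes a session capacity check that kicks excess players as "Server Full", then updates the session.
; CreatActor then spawns a Warrior or ThirdPersonCharacter at an index-named player start for each PC_Game not yet set up, which possesses it.
; DebugMode skips session handling and spawns once three players are present.
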(event EventHandleStartingNewPlayer
  (params (NewPlayer :type Player%20Controller%20Object%20Reference))
  (if (not (Variables|Default|GetDebugMode))
    ;[1 1 1] On Starting New Player // Remove client if to many client and create player character
    (Utilities|Array|AddUnique (Variables|Default|GetplayerControllers) NewPlayer)
    (Utilities|FlowControl|RetriggerableDelay 2.0)
    (bind (_numconnections _numprivateconnections _bislan _bisdedicated _ballowinvites _ballowjoininprogress _bisanticheatenabled _builduniqueid _extrasettings) (Class|AdvancedSessionsLibrary|GetSessionSettings)
      (:OnSuccess
        (if (> (Utilities|Array|Length (Variables|/Script/Engine.GameStateBase|GetPlayerArray (Game|GetGameState))) _numconnections)
          (bind (_arrayindex _arrayelement) (Utilities|Array|ReverseforEachLoop (Variables|Default|GetplayerControllers))
            (:LoopBody
              (if (>= _arrayindex _numconnections)
                (Class|AdvancedSessionsLibrary|KickPlayer _arrayelement "Server Full")))
            (:Completed
              (|UpdateSession _extrasettings _numconnections 0 false false false true false :!label _label
                (:OnSuccess
                  (for (_array_element _array_index) (Variables|Default|GetplayerControllers)
                    (bind _aspc_game (Utilities|Casting|CastToPC_Game _array_element))
                    (if (not (Variables|/Game/Levels/Game/PC_Game.PC_Game_C|GetIsControllerSetUP _aspc_game))
                      (bind _bp_tpc (CallFunction|CreatActor (Variables|/Game/Levels/Game/PC_Game.PC_Game_C|GetCharacterSelection _aspc_game) (Transformation|GetActorTransform (Class|GameModeBase|FindPlayerStart _aspc_game (Utilities|String|ToString(Integer) _array_index)))))
                      (Pawn|Possess _aspc_game _bp_tpc)
                      (Variables|/Game/Levels/Game/PC_Game.PC_Game_C|SetIsControllerSetUP _aspc_game true)))))))
          (else
            (goto _label)))))
    (else
      ;[1 1 1] For Debug
      (Utilities|Array|AddUnique (Variables|Default|GetplayerControllers) NewPlayer)
      (if (== (Utilities|Array|Length (Variables|/Script/Engine.GameStateBase|GetPlayerArray (Game|GetGameState))) 3)
        (for (_array_element_2 _array_index_2) (Variables|Default|GetplayerControllers)
          (bind _aspc_game_2 (Utilities|Casting|CastToPC_Game _array_element_2))
          (if (not (Variables|/Game/Levels/Game/PC_Game.PC_Game_C|GetIsControllerSetUP _aspc_game_2))
            (bind _bp_tpc_2 (CallFunction|CreatActor (Variables|/Game/Levels/Game/PC_Game.PC_Game_C|GetCharacterSelection _aspc_game_2) (Transformation|GetActorTransform (Class|GameModeBase|FindPlayerStart _aspc_game_2 (Utilities|String|ToString(Integer) _array_index_2)))))
            (Pawn|Possess _aspc_game_2 _bp_tpc_2)
            (Variables|/Game/Levels/Game/PC_Game.PC_Game_C|SetIsControllerSetUP _aspc_game_2 true)))))))

(event EventOnLogout
  (params (ExitingController :type Controller%20Object%20Reference))
  ;[1 1 1] OnLogout or OnKick
  (bind _asplayer_controller (Utilities|Casting|CastToPlayerController ExitingController))
  (Utilities|Array|RemoveItem (Variables|Default|GetplayerControllers) _asplayer_controller))

(fn ConstructionScript)

(fn CreatActor
  (params (Enum :type ENUM_Player_character_selection%20Enum :default "NewEnumerator0") (Transform :type Transform))
  (Utilities|FlowControl|Sequence
    (:then_0
      (if (Utilities|Enum|Equal(Enum) Enum "NewEnumerator0")
        (bind _returnvalue (Game|SpawnActorfromClass "/Game/ThirdPersonBP/BP_TPC_Warrior.BP_TPC_Warrior_C" Transform "Undefined" 0 0))
        (return _returnvalue)))
    (:then_1
      (if (Utilities|Enum|Equal(Enum) Enum "NewEnumerator1")
        (bind _returnvalue_2 (Game|SpawnActorfromClass "/Game/ThirdPersonBP/ThirdPersonCharacter.ThirdPersonCharacter_C" Transform "Undefined" 0 0))
        (return _returnvalue_2)))))