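; PC_Game is a player controller for the game level that passes the player's saved character choice on for storage on the controller.
; On BeginPlay, the local controller loads the SaveMenu save and sends its character selection through S_SendCharacterSelection, which stores it in CharacterSelection.
; The CharacterSelection OnRep is empty, and UnPossess clears the controller setup flag.
; Pressing Enter on the server runs a server travel to the Game map.
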(event Custom|S_SendCharacterSelection
  (params (CharacterSelection :type ENUM_Player_character_selection%20Enum :default "NewEnumerator0"))
  (Variables|Default|SetCharacterSelection CharacterSelection))

(event EventBeginPlay
  (if (Pawn|IsLocalController)
    (bind _returnvalue (SaveGame|LoadGamefromSlot "SaveMenu"))
    (bind _asbp_save_menu (Utilities|Casting|CastToBP_SaveMenu _returnvalue))
    (CallFunction|SSendCharacterSelection (Variables|/Game/Levels/Menu/BP_SaveMenu.BP_SaveMenu_C|GetPlayerCharacterSelec _asbp_save_menu))))

(event EventUnPossess
  (params (UnpossessedPawn :type Pawn%20Object%20Reference))
  (Variables|Default|SetIsControllerSetUP false))

(event Input|KeyboardEvents|Enter
  (params (Key :type Key%20Structure :default "None"))
  (:Pressed
    (if (Networking|IsServer)
      (Development|ExecuteConsoleCommand "serverTravel Game" 0))))

(fn ConstructionScript)

(fn OnRepCharacterSelection)